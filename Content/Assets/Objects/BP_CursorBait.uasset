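; BP_CursorBait is an actor that follows the mouse cursor across a designated hittable surface.
; Each tick it deprojects the cursor to world space and line traces along that direction using the WaterBodyCollision profile.
; When the trace hits the HittablePlane actor, it moves to the hit point's X and Y while keeping its own height.
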(event EventBeginPlay)

(event Collision|EventActorBeginOverlap
  (params (OtherActor :type Actor%20Object%20Reference)))

(event EventTick
  (params (DeltaSeconds :type Float%20%28single-precision%29))
  (bind _returnvalue (Game|GetPlayerController 0))
  (bind (_worldlocation _worlddirection) (Game|Player|ConvertMouseLocationToWorldSpace _returnvalue))
  (bind (_outhit _returnvalue_2) (Class|KismetSystemLibrary|LineTraceSinglebyProfile _worldlocation (+ _worldlocation (* _worlddirection (Variables|Default|Getdistance))) "WaterBodyCollision" false 0 "None" true))
  (if _returnvalue_2
    (if (== (.HitActor (Collision|BreakHitResult _outhit)) (Variables|Default|GethittablePlane))
      (Transformation|SetActorLocation (Math|Vector|MakeVector (.X (Math|Vector|BreakVector (.Location (Collision|BreakHitResult _outhit)))) (.Y (Math|Vector|BreakVector (.Location (Collision|BreakHitResult _outhit)))) (.Z (Math|Vector|BreakVector (Transformation|GetActorLocation)))) false false))))

(fn ConstructionScript)