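; BP_CursorBait is a bait cursor actor that follows where the player's camera points on a designated hittable plane.
; Each Tick it line traces from the camera along its forward vector for a set Distance, using the WaterBodyCollision profile.
; When the trace hits HittablePlane, the actor moves to the hit's X and Y while keeping its own height.
; A debug camera-channel trace is left unconnected.
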(event EventBeginPlay)

(event Collision|EventActorBeginOverlap
  (params (OtherActor :type Actor%20Object%20Reference)))

(event EventTick
  (params (DeltaSeconds :type Float%20%28single-precision%29))
  (bind _returnvalue (Game|GetPlayerCameraManager 0))
  (bind _returnvalue_2 (Camera|GetCameraLocation _returnvalue))
  (bind (_outhit _returnvalue_3) (Class|KismetSystemLibrary|LineTraceSinglebyProfile _returnvalue_2 (+ _returnvalue_2 (* (Transformation|GetActorForwardVector _returnvalue) (Variables|Default|Getdistance))) "WaterBodyCollision" false 0 "None" true))
  (if _returnvalue_3
    (if (== (.HitActor (Collision|BreakHitResult _outhit)) (Variables|Default|GethittablePlane))
      (Transformation|SetActorLocation (Math|Vector|MakeVector (.X (Math|Vector|BreakVector (.Location (Collision|BreakHitResult _outhit)))) (.Y (Math|Vector|BreakVector (.Location (Collision|BreakHitResult _outhit)))) (.Z (Math|Vector|BreakVector (Transformation|GetActorLocation)))) false false))))

(fn ConstructionScript)