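; BP_MenuLogicCredit is a menu entry actor, by its name the Credits option, that highlights when the cursor bait actor overlaps it.
; Begin and end overlap events filter for CursorBait, switch the TextRender between selected and unselected colors, and set IsOverlapped.
; BeginPlay starts it unselected.
; The file only tracks hover state and contains no click or activation logic.
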(event EventBeginPlay
  (Variables|Default|SetisOverlapped false)
  (Rendering|Components|TextRender|SetTextRenderColor (Variables|Default|GetTextRender) (Variables|Default|GetunselectedColor))
  (Variables|Default|SetisOverlapped false))

(event Collision|EventActorBeginOverlap
  (params (OtherActor :type Actor%20Object%20Reference))
  (if (== OtherActor (Variables|Default|GetCursorBait))
    (Rendering|Components|TextRender|SetTextRenderColor (Variables|Default|GetTextRender) (Variables|Default|GetselectedColor))
    (Variables|Default|SetisOverlapped true)))

(event EventTick
  (params (DeltaSeconds :type Float%20%28single-precision%29)))

(event Collision|EventActorEndOverlap
  (params (OtherActor :type Actor%20Object%20Reference))
  (if (== (Variables|Default|GetCursorBait) OtherActor)
    (Rendering|Components|TextRender|SetTextRenderColor (Variables|Default|GetTextRender) (Variables|Default|GetunselectedColor))
    (Variables|Default|SetisOverlapped false)))

(fn ConstructionScript)